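; WeaponFire is an actor Blueprint that fires a cannon shot with effects.
; EventFire spawns a muzzle emitter and a Bullet at the actor's position, forcing the spawn despite collision, and plays the cannon sound at the world origin.
; BeginPlay enables input from the first player controller.
; A setter stores the team, which the firing logic does not read, and collision-related nodes sit unconnected.
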(event EventBeginPlay
  (Input|EnableInput (Game|GetPlayerController 0)))

(event EventEventFire
  (Effects|SpawnEmitteratLocation "/Game/Particles/Cannon_Fire.Cannon_Fire" (Transformation|GetActorLocation) "0,0.000000, 0")
  (Game|SpawnActorfromClass "/Game/Blueprints/Bullet.Bullet_C" (Transformation|GetActorTransform) true 0)
  (Audio|PlaySoundatLocation "/Game/Sounds/Cannon_Fire_Cue.Cannon_Fire_Cue" "0, 0, 0"))

(fn ConstructionScript)

(fn SetWeaponFireTeam
  (params (NewParam :type TEAM%20Enum :default "Team_Red"))
  (Variables|Default|Setm_teams NewParam))