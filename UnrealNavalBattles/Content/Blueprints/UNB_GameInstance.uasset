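; Game instance Blueprint that drives front-end flow and LAN multiplayer sessions, from main menu and server list to loading screen and play.
; A state machine in TransitionToState removes the current screen, or destroys the session when leaving Playing, before switching state.
; Each menu event lazily creates and caches its widget, then shows it with UI-only input.
; Hosting creates a two-connection LAN session and opens map0 as listen server; joining uses a selected search result.
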(event Custom|ShowServerListEvent
  (bind _returnvalue (Game|GetPlayerController 0))
  ;[1 1 1] Show ServerList
  (Utilities|TransitiontoState "NewEnumerator4"
    (:newState
      (Utilities|IsValid (Variables|Default|GetServerList)
        (:Is%20Valid
          _)
        (:Is%20Not%20Valid
          (bind _returnvalue_2 (UserInterface|CreateWidget "/Game/Blueprints/ServerList.ServerList_C" _returnvalue))
          (Variables|Default|SetServerList _returnvalue_2)))
      (UserInterface|Viewport|AddtoViewport (Variables|Default|GetServerList))
      (Input|SetInputModeUIOnly _returnvalue (Variables|Default|GetServerList) false))))

(event Custom|HostGameEvent
  ;[1 1 1] HOST GAME
  (CallFunction|ShowLoadingScreen)
  (Utilities|FlowControl|Delay 0.0)
  (|Session (Game|GetPlayerController 0) 2 true
    (:OnSuccess
      (Game|OpenLevel(byName) "map0" true "listen"))
    (:OnFailure
      (Development|PrintString "Create Session FAILED"))))

(event Custom|ShowLoadingScreen
  (bind _returnvalue (Game|GetPlayerController 0))
  ;[1 1 1] Show Loading screen- Called when hosting or joining
  (Utilities|TransitiontoState "NewEnumerator3"
    (:newState
      (Utilities|IsValid (Variables|Default|GetLoadingScreen)
        (:Is%20Valid
          _)
        (:Is%20Not%20Valid
          (bind _returnvalue_2 (UserInterface|CreateWidget "/Game/Blueprints/LoadingScreen.LoadingScreen_C" _returnvalue))
          (Variables|Default|SetLoadingScreen _returnvalue_2)))
      (UserInterface|Viewport|AddtoViewport (Variables|Default|GetLoadingScreen))
      (Input|SetInputModeUIOnly _returnvalue (Variables|Default|GetLoadingScreen) false))))

(event Custom|Start%20Playing%20State
  (Utilities|TransitiontoState "NewEnumerator2"))

(event Custom|ShowMainMenuEvent
  (bind _returnvalue (Game|GetPlayerController 0))
  ;[1 1 1] ON StartUp
  (Utilities|IsCurrentState "NewEnumerator2"
    (:True
      (Game|OpenLevel(byName) "MainMenu"))
    (:False
      _))
  (Utilities|TransitiontoState "NewEnumerator1"
    (:Same%20State
      (Development|PrintString "Hello"))
    (:newState
      (Utilities|IsValid (Variables|Default|GetMenu)
        (:Is%20Valid
          _)
        (:Is%20Not%20Valid
          (bind _returnvalue_2 (UserInterface|CreateWidget "/Game/Blueprints/Menu.Menu_C" _returnvalue))
          (Variables|Default|SetMenu _returnvalue_2)))
      (Input|SetInputModeUIOnly _returnvalue (Variables|Default|GetMenu) false)
      (UserInterface|Viewport|AddtoViewport (Variables|Default|GetMenu)))))

(event Custom|JoinFromServerListEvent
  (params (NewParam :type Blueprint%20Session%20Result%20Structure))
  ;[1 1 1] Join From Server List
  (CallFunction|ShowLoadingScreen)
  (|JoinSession (Game|GetPlayerController 0) NewParam
    (:OnSuccess
      (Development|PrintString (Class|FindSessionsCallbackProxy|GetServerName NewParam)))
    (:OnFailure
      (Development|PrintString "Failed to join session"))))

(fn BeginPlayShowMainMenu
  (Utilities|IsCurrentState "NewEnumerator0"
    (:True
      (CallFunction|ShowMainMenuEvent))))