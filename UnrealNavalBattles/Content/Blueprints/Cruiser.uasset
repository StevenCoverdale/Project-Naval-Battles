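; Cruiser is a unit Blueprint that carries eight weapon child actors and assigns each of them the Cruiser's team.
; The Construction Script casts each ChildActor to WeaponFire in sequence and passes MTeam to it through SetWeaponFireTeam.
; The casts are chained, so one failed cast leaves all later weapons without a team assignment from this script.
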(fn ConstructionScript
  (bind _asweapon_fire (Utilities|Casting|CastToWeaponFire (Variables|/Script/Engine.ChildActorComponent|GetChildActor (Variables|Default|GetChildActor1))))
  (Default|SetWeaponFireTeam _asweapon_fire (Variables|Default|Getm_team))
  (bind _asweapon_fire_2 (Utilities|Casting|CastToWeaponFire (Variables|/Script/Engine.ChildActorComponent|GetChildActor (Variables|Default|GetChildActor2))))
  (Default|SetWeaponFireTeam _asweapon_fire_2 (Variables|Default|Getm_team))
  (bind _asweapon_fire_3 (Utilities|Casting|CastToWeaponFire (Variables|/Script/Engine.ChildActorComponent|GetChildActor (Variables|Default|GetChildActor3))))
  (Default|SetWeaponFireTeam _asweapon_fire_3 (Variables|Default|Getm_team))
  (bind _asweapon_fire_4 (Utilities|Casting|CastToWeaponFire (Variables|/Script/Engine.ChildActorComponent|GetChildActor (Variables|Default|GetChildActor4))))
  (Default|SetWeaponFireTeam _asweapon_fire_4 (Variables|Default|Getm_team))
  (bind _asweapon_fire_5 (Utilities|Casting|CastToWeaponFire (Variables|/Script/Engine.ChildActorComponent|GetChildActor (Variables|Default|GetChildActor5))))
  (Default|SetWeaponFireTeam _asweapon_fire_5 (Variables|Default|Getm_team))
  (bind _asweapon_fire_6 (Utilities|Casting|CastToWeaponFire (Variables|/Script/Engine.ChildActorComponent|GetChildActor (Variables|Default|GetChildActor6))))
  (Default|SetWeaponFireTeam _asweapon_fire_6 (Variables|Default|Getm_team))
  (bind _asweapon_fire_7 (Utilities|Casting|CastToWeaponFire (Variables|/Script/Engine.ChildActorComponent|GetChildActor (Variables|Default|GetChildActor7))))
  (Default|SetWeaponFireTeam _asweapon_fire_7 (Variables|Default|Getm_team))
  (bind _asweapon_fire_8 (Utilities|Casting|CastToWeaponFire (Variables|/Script/Engine.ChildActorComponent|GetChildActor (Variables|Default|GetChildActor8))))
  (Default|SetWeaponFireTeam _asweapon_fire_8 (Variables|Default|Getm_team)))